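; Sound trigger Blueprint that plays a bubble sound while something overlaps its box volume.
; Begin overlap sets a flag and plays the sound at the audio component's location, also raising that component's volume multiplier.
; While the flag is set, Tick feeds a Delay that repeats this about every four seconds.
; End overlap clears the flag without cancelling a pending Delay, and overlapping actors are not filtered.
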(event `self.Box.OnComponentBeginOverlap`
  (params (OverlappedComponent :type "PrimitiveComponent Object Reference") (OtherActor :type "Actor Object Reference") (OtherComp :type "PrimitiveComponent Object Reference") (OtherBodyIndex :type Integer) (bFromSweep :type Boolean) (SweepResult :type "HitResult Structure (by ref)"))
  (set `self.isOnBox` true)
  (`AudioComponent.SetVolumeMultiplier` (`self.AudioComponent`) 2.0)
  (`GameplayStatics.PlaySoundAtLocation` "/Game/Level_Mathieu/Sounds/Bruit_Bulle_0.Bruit_Bulle_0" (`SceneComponent.K2_GetComponentLocation` (`self.AudioComponent`)) (struct) 1.0 1.0 0.0 null null null null))

(event `self.ReceiveTick`
  (params (DeltaSeconds :type "Float (single-precision)"))
  (if (`self.isOnBox`)
    (`KismetSystemLibrary.Delay` 4.0)
    (`AudioComponent.SetVolumeMultiplier` (`self.AudioComponent`) 2.0)
    (`GameplayStatics.PlaySoundAtLocation` "/Game/Level_Mathieu/Sounds/Bruit_Bulle_0.Bruit_Bulle_0" (`SceneComponent.K2_GetComponentLocation` (`self.AudioComponent`)) (struct) 1.0 1.0 0.0 null null null null)))

(event `self.Box.OnComponentEndOverlap`
  (params (OverlappedComponent :type "PrimitiveComponent Object Reference") (OtherActor :type "Actor Object Reference") (OtherComp :type "PrimitiveComponent Object Reference") (OtherBodyIndex :type Integer))
  (set `self.isOnBox` false))

(fn `UserConstructionScript`)