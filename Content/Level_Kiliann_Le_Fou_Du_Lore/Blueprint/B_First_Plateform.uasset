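; B_First_Plateform is a platform actor whose Cube falls under physics the first time the player pawn hits it.
; A DoOnce limits the sequence to one run, turning on physics simulation and asking HUD_ to create a dialogue from Diag.
; After a short delay, physics turns off and MoveComponentTo returns the cube to its BeginPlay position, saved in world space but passed as a relative target.
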(event `self.ReceiveBeginPlay`
  (set `self.Pos` (`SceneComponent.K2_GetComponentLocation` (`self.Cube`))))

(event `self.ReceiveTick`
  (params (DeltaSeconds :type "Float (single-precision)")))

(event `self.Cube.OnComponentHit`
  (params (HitComponent :type "PrimitiveComponent Object Reference") (OtherActor :type "Actor Object Reference") (OtherComp :type "PrimitiveComponent Object Reference") (NormalImpulse :type "Vector Structure") (Hit :type "HitResult Structure (by ref)"))
  (bind _cube (`self.Cube`))
  (if (== OtherActor (`GameplayStatics.GetPlayerPawn` 0))
    (`/Engine/EditorBlueprintResources/StandardMacros.DoOnce` false
      (:`Completed`
        (`PrimitiveComponent.SetSimulatePhysics` (`self.Cube`) true)
        (`|ExecutionSequence`
          (:`then_0`
            (`KismetSystemLibrary.Delay` 4.0)
            (`PrimitiveComponent.SetSimulatePhysics` _cube false)
            (`KismetSystemLibrary.MoveComponentTo` _cube (`self.Pos`) (struct) false false 0.5))
          (:`then_1`
            (bind _ashud_ (cast `/Game/Level_Adrien/HUD_` (`PlayerController.GetHUD` (`GameplayStatics.GetPlayerController` 0))))
            (`/Game/Level_Adrien/HUD_.CreateDialogue` _ashud_ (`self.Diag`))))))))

(fn `UserConstructionScript`)