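; Level platform actor that, once the player pawn first hits its cube, shows a dialogue and starts shifting back and forth.
; BeginPlay stores the cube's start location and a second point offset along negative Y.
; A DoOnce on the hit creates the HUD_ dialogue, then an endless Delay loop snaps the cube between both points at fixed intervals, without interpolation.
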(event `self.ReceiveBeginPlay`
  (bind _output_get (set `self.Pos1` (`SceneComponent.K2_GetComponentLocation` (`self.Cube`))))
  (set `self.Pos2` (`KismetMathLibrary.MakeVector` (.x _output_get) (- (.y _output_get) 620.0) (.z _output_get))))

(event `self.Cube.OnComponentHit`
  (params (HitComponent :type "PrimitiveComponent Object Reference") (OtherActor :type "Actor Object Reference") (OtherComp :type "PrimitiveComponent Object Reference") (NormalImpulse :type "Vector Structure") (Hit :type "HitResult Structure (by ref)"))
  (if (== OtherActor (`GameplayStatics.GetPlayerPawn` 0))
    (`/Engine/EditorBlueprintResources/StandardMacros.DoOnce` false
      (:`Completed`
        (bind _ashud_ (cast `/Game/Level_Adrien/HUD_` (`PlayerController.GetHUD` (`GameplayStatics.GetPlayerController` 0))))
        (`/Game/Level_Adrien/HUD_.CreateDialogue` _ashud_ (`self.Diag`))
        (if (== (`SceneComponent.K2_GetComponentLocation` (`self.Cube`)) (`self.Pos1`)) :!label _label
          (`SceneComponent.K2_SetWorldTransform` (`self.Cube`) (`KismetMathLibrary.MakeTransform` (`self.Pos2`)) false false)
          (`KismetSystemLibrary.Delay` 5.0)
          (goto _label)
          (else
            (`SceneComponent.K2_SetWorldTransform` (`self.Cube`) (`KismetMathLibrary.MakeTransform` (`self.Pos1`)) false false)
            (`KismetSystemLibrary.Delay` 5.0)
            (goto _label)))))))

(fn `UserConstructionScript`)