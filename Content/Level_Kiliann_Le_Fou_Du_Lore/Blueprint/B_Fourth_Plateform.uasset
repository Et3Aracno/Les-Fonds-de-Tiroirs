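; Fourth platform Blueprint: an invisible cube that reveals itself and triggers dialogue when the player hits it.
; The cube's visibility is turned off on BeginPlay, while its component hit event still detects the player pawn.
; A DoOnce gate makes the first player hit show the cube and pass its Diag data to the player HUD's CreateDialogue.
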(event `self.ReceiveBeginPlay`
  (`SceneComponent.SetVisibility` (`self.Cube`) false false))

(event `self.Cube.OnComponentHit`
  (params (HitComponent :type "PrimitiveComponent Object Reference") (OtherActor :type "Actor Object Reference") (OtherComp :type "PrimitiveComponent Object Reference") (NormalImpulse :type "Vector Structure") (Hit :type "HitResult Structure (by ref)"))
  (if (== OtherActor (`GameplayStatics.GetPlayerPawn` 0))
    (`/Engine/EditorBlueprintResources/StandardMacros.DoOnce` false
      (:`Completed`
        (`SceneComponent.SetVisibility` (`self.Cube`) true false)
        (bind _ashud_ (cast `/Game/Level_Adrien/HUD_` (`PlayerController.GetHUD` (`GameplayStatics.GetPlayerController` 0))))
        (`/Game/Level_Adrien/HUD_.CreateDialogue` _ashud_ (`self.Diag`))))))

(fn `UserConstructionScript`)