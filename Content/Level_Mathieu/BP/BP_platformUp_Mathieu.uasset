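; BP_platformUp_Mathieu is a moving platform that activates when the player character's ScoreMathieu equals 3.
; Any actor beginning overlap triggers a check of player 0's score, then makes Cube visible and moves it to PosEnd2.
; Any end overlap moves Cube back to PosEnd1 without a score check or hiding it, with Alpha as the duration of both moves.
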(event `self.ReceiveActorBeginOverlap`
  (params (OtherActor :type "Actor Object Reference"))
  (bind _asbp_first_person_character_mathieu (cast `/Game/Level_Mathieu/BP/BP_FirstPersonCharacter_Mathieu` (`GameplayStatics.GetPlayerCharacter` 0)))
  (bind _returnvalue (== (`/Game/Level_Mathieu/BP/BP_FirstPersonCharacter_Mathieu.Score_Mathieu` _asbp_first_person_character_mathieu) 3))
  (if _returnvalue
    (`SceneComponent.SetVisibility` (`self.Cube`) _returnvalue false)
    (`KismetSystemLibrary.MoveComponentTo` (`self.Cube`) (`SceneComponent.RelativeLocation` (`self.posEnd2`)) (struct) false false (`self.Alpha`))))

(event `self.ReceiveActorEndOverlap`
  (params (OtherActor :type "Actor Object Reference"))
  (`KismetSystemLibrary.MoveComponentTo` (`self.Cube`) (`SceneComponent.RelativeLocation` (`self.posEnd1`)) (struct) false false (`self.Alpha`)))

(fn `UserConstructionScript`)