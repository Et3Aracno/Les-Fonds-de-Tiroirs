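; Dialogue trigger volume that times a banana spawn to the dialogue as the player enters its box.
; On player overlap, it asks the HUD for the duration of its DialogueStruct and waits until four seconds before that time elapses.
; It then searches all BP_Spawner actors and fires the first whose spawner type is Banana, matched by enum name string.
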(event `self.Box.OnComponentBeginOverlap`
  (params (OverlappedComponent :type "PrimitiveComponent Object Reference") (OtherActor :type "Actor Object Reference") (OtherComp :type "PrimitiveComponent Object Reference") (OtherBodyIndex :type Integer) (bFromSweep :type Boolean) (SweepResult :type "HitResult Structure (by ref)"))
  (if (== OtherActor (`GameplayStatics.GetPlayerPawn` 0))
    (bind _ashud_ (cast `/Game/Level_Adrien/HUD_` (`PlayerController.GetHUD` (`GameplayStatics.GetPlayerController` 0))))
    (`KismetSystemLibrary.Delay` (- (`/Game/Level_Adrien/HUD_.GetDialoguTime` _ashud_ (`self.DialogueStruct`)) 4.0))
    (bind _outactors (`GameplayStatics.GetAllActorsOfClass` "/Game/Level_Adrien/BP_Spawner.BP_Spawner_C"))
    (for _array_element _outactors
      (if (`KismetStringLibrary.EqualEqual_StrStr` (`|GetEnumeratorNameAsString` (`/Game/Level_Adrien/BP_Spawner.spawnerType` _array_element)) "Banana")
        (`/Game/Level_Adrien/BP_Spawner.SpawnActor` _array_element)
        (break)))))

(fn `UserConstructionScript`
  (`parent.UserConstructionScript`))