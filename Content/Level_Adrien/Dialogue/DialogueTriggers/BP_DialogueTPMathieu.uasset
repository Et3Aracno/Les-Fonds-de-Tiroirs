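; BP_DialogueTPMathieu is a dialogue trigger that teleports the player and then shows a joke "wrong level" title on screen.
; When the player pawn overlaps the Box, it asks the HUD for the duration of its DialogueStruct and waits slightly longer than that.
; It then moves the player to the Cube component's location with zero rotation and, after a further pause, has the HUD create the title.
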(event `self.Box.OnComponentBeginOverlap`
  (params (OverlappedComponent :type "PrimitiveComponent Object Reference") (OtherActor :type "Actor Object Reference") (OtherComp :type "PrimitiveComponent Object Reference") (OtherBodyIndex :type Integer) (bFromSweep :type Boolean) (SweepResult :type "HitResult Structure (by ref)"))
  (bind _returnvalue (`GameplayStatics.GetPlayerPawn` 0))
  (if (== OtherActor _returnvalue)
    (bind _ashud_ (cast `/Game/Level_Adrien/HUD_` (`PlayerController.GetHUD` (`GameplayStatics.GetPlayerController` 0))))
    (`KismetSystemLibrary.Delay` (+ (`/Game/Level_Adrien/HUD_.GetDialoguTime` _ashud_ (`self.DialogueStruct`)) 1.0))
    (`self.K2_TeleportTo` :`self` _returnvalue :`DestLocation` (`SceneComponent.K2_GetComponentLocation` (`self.Cube`)))
    (`KismetSystemLibrary.Delay` 15.0)
    (`/Game/Level_Adrien/HUD_.CreateTitle` _ashud_ "Wrong Level my bad")))

(fn `UserConstructionScript`
  (`parent.UserConstructionScript`))