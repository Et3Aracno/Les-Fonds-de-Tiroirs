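; BP_Button is a one-shot interactable button that plays a dialogue and then makes the custom door passable.
; On Interact, a DoOnce gate dips the cube down and back up, waits, then starts DialogueStructure through the player's HUD_.
; A second delay, derived from the dialogue's duration minus a fixed offset, precedes disabling Door collision on the BP_CustomDoor found by GetActorOfClass, plus a debug print.
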(event `/Game/BPI_Interact.Interact`
  (bind _cube (`self.Cube`))
  (bind _dialoguestructure (`self.DialogueStructure`))
  (bind _relativelocation (`SceneComponent.RelativeLocation` _cube))
  (`/Engine/EditorBlueprintResources/StandardMacros.DoOnce` false
    (:`Completed`
      (`KismetSystemLibrary.MoveComponentTo` _cube (- _relativelocation (0.0 0.0 20.0)) (struct) false false 0.2)
      (`KismetSystemLibrary.MoveComponentTo` _cube (+ _relativelocation (0.0 0.0 20.0)) (struct) false false 0.2)
      (`KismetSystemLibrary.Delay` 4.0)
      (bind _ashud_ (cast `/Game/Level_Adrien/HUD_` (`PlayerController.GetHUD` (`GameplayStatics.GetPlayerController` 0))))
      (`/Game/Level_Adrien/HUD_.CreateDialogue` _ashud_ _dialoguestructure)
      (`KismetSystemLibrary.Delay` (- (`/Game/Level_Adrien/HUD_.GetDialoguTime` _ashud_ _dialoguestructure) 4.0))
      (bind _returnvalue (`GameplayStatics.GetActorOfClass` "/Game/Level_Adrien/BP_CustomDoor.BP_CustomDoor_C"))
      (`PrimitiveComponent.SetCollisionEnabled` (`/Game/Level_Adrien/BP_CustomDoor.Door` _returnvalue) "NoCollision")
      (`KismetSystemLibrary.PrintString` "Hello"))))

(fn `UserConstructionScript`)