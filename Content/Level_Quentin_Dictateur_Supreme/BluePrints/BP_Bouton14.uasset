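; BP_Bouton14 is a one-shot interactable lever that reveals two other wall buttons and starts a continuous rain of spawned levers.
; An overlap box shows the widget and tracks player presence; both linked button cubes start hidden.
; Interact tilts the lever, enables its physics, reveals Bouton0 and Bouton13, sets the dialogue flag and plays a bonk.
; It also sets SPAWN, so Tick repeatedly spawns BP_Levers at random Spawn actors, throttled by a short Delay.
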(event `self.ReceiveTick`
  (params (DeltaSeconds :type "Float (single-precision)"))
  (if (`self.SPAWN!`)
    (`KismetSystemLibrary.Delay` 0.2)
    (`self.SpawnLevers`)))

(event `ViewButton_13`
  (`SceneComponent.SetVisibility` (`/Game/Level_Quentin_Dictateur_Supreme/BluePrints/BP_Bouton13.Cube_Sur_Mur` (`self.Bouton 13`)) true true))

(event `ViewButton_0`
  (`SceneComponent.SetVisibility` (`/Game/Level_Quentin_Dictateur_Supreme/BluePrints/BP_Bouton0.Cube_Sur_Mur` (`self.Bouton 0`)) true true))

(event `/Game/BPI_Interact.Interact`
  (`/Engine/EditorBlueprintResources/StandardMacros.DoOnce` false
    (:`Completed`
      (`KismetSystemLibrary.MoveComponentTo` (`self.Levier`) (0.0 0.0 15.0) (struct :`Roll` -40.0))
      (`PrimitiveComponent.SetSimulatePhysics` (`self.Levier`) true)
      (`self.ViewButton_0`)
      (`self.ViewButton_13`)
      (set `self.SPAWN!` true)
      (set `self.Dialogue` true)
      (`/Engine/EditorBlueprintResources/StandardMacros.DoOnce` false
        (:`Completed`
          (`GameplayStatics.PlaySound2D` "/Game/Level_Quentin_Dictateur_Supreme/Assets/BONK.BONK" 1.0 1.0 0.0 null null))))))

(event `self.ReceiveBeginPlay`
  (`SceneComponent.SetVisibility` (`self.Widget`) false false)
  (`SceneComponent.SetVisibility` (`/Game/Level_Quentin_Dictateur_Supreme/BluePrints/BP_Bouton13.Cube_Sur_Mur` (`self.Bouton 13`)) false true)
  (`SceneComponent.SetVisibility` (`/Game/Level_Quentin_Dictateur_Supreme/BluePrints/BP_Bouton0.Cube_Sur_Mur` (`self.Bouton 0`)) false true))

(event `self.Box1.OnComponentBeginOverlap`
  (params (OverlappedComponent :type "PrimitiveComponent Object Reference") (OtherActor :type "Actor Object Reference") (OtherComp :type "PrimitiveComponent Object Reference") (OtherBodyIndex :type Integer) (bFromSweep :type Boolean) (SweepResult :type "HitResult Structure (by ref)"))
  (set `self.IsInBox?` true)
  (`SceneComponent.SetVisibility` (`self.Widget`) true false))

(event `self.Box1.OnComponentEndOverlap`
  (params (OverlappedComponent :type "PrimitiveComponent Object Reference") (OtherActor :type "Actor Object Reference") (OtherComp :type "PrimitiveComponent Object Reference") (OtherBodyIndex :type Integer))
  (set `self.IsInBox?` false)
  (`SceneComponent.SetVisibility` (`self.Widget`) false false))

(fn `SpawnLevers`
  (`|SpawnActorFromClass` "/Game/Level_Quentin_Dictateur_Supreme/BluePrints/BP_Levers.BP_Levers_C" (`self.GetTransform` (`|GetArrayItem` (`self.Spawn`) (`KismetMathLibrary.RandomIntegerInRange` 0 (- (`KismetArrayLibrary.Array_Length` (`self.Spawn`)) 1)))) "Undefined" "MultiplyWithRoot" null null))

(fn `UserConstructionScript`)