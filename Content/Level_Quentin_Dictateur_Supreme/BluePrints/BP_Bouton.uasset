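; BP_Bouton is a single-use interactable lever (Levier) that the player activates with the E key.
; Overlapping Box1 sets IsInBox and shows a prompt widget, which is hidden at BeginPlay and on leaving.
; Tick polls the key while inside; a DoOnce gate moves and tilts the lever, then enables physics simulation on it.
; Nothing else is triggered by the lever in this graph.
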(event `self.ReceiveTick`
  (params (DeltaSeconds :type "Float (single-precision)"))
  (if (`self.IsInBox?`)
    (if (`PlayerController.IsInputKeyDown` (`GameplayStatics.GetPlayerController` 0) "E")
      (`/Engine/EditorBlueprintResources/StandardMacros.DoOnce` false
        (:`Completed`
          (`KismetSystemLibrary.MoveComponentTo` (`self.Levier`) (0.0 0.0 15.0) (struct :`Roll` -40.0))
          (`PrimitiveComponent.SetSimulatePhysics` (`self.Levier`) true))))))

(event `self.ReceiveBeginPlay`
  (`SceneComponent.SetVisibility` (`self.Widget`) false false))

(event `self.Box1.OnComponentBeginOverlap`
  (params (OverlappedComponent :type "PrimitiveComponent Object Reference") (OtherActor :type "Actor Object Reference") (OtherComp :type "PrimitiveComponent Object Reference") (OtherBodyIndex :type Integer) (bFromSweep :type Boolean) (SweepResult :type "HitResult Structure (by ref)"))
  (set `self.IsInBox?` true)
  (`SceneComponent.SetVisibility` (`self.Widget`) true false))

(event `self.Box1.OnComponentEndOverlap`
  (params (OverlappedComponent :type "PrimitiveComponent Object Reference") (OtherActor :type "Actor Object Reference") (OtherComp :type "PrimitiveComponent Object Reference") (OtherBodyIndex :type Integer))
  (set `self.IsInBox?` false)
  (`SceneComponent.SetVisibility` (`self.Widget`) false false))

(fn `UserConstructionScript`)