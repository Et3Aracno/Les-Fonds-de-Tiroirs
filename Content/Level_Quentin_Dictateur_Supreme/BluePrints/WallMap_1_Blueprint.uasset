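; Wall map Blueprint that acts as the level's ending trigger, moving the player to Level_EndLobby.
; When the player pawn overlaps its box while the Dialogue's door permission is set, a DoOnce fires.
; It swaps the mesh to a Flash material, shows the end interface widget and plays a flashbang sound, then opens the end lobby after a short delay.
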(event `self.Box.OnComponentBeginOverlap`
  (params (OverlappedComponent :type "PrimitiveComponent Object Reference") (OtherActor :type "Actor Object Reference") (OtherComp :type "PrimitiveComponent Object Reference") (OtherBodyIndex :type Integer) (bFromSweep :type Boolean) (SweepResult :type "HitResult Structure (by ref)"))
  (if (and (== OtherActor (`GameplayStatics.GetPlayerPawn` 0)) (`/Game/Level_Quentin_Dictateur_Supreme/Dialogue/BP_Dialogue.GivePermissionsDoor` (`self.Dialogue`)))
    (`/Engine/EditorBlueprintResources/StandardMacros.DoOnce` false
      (:`Completed`
        (`PrimitiveComponent.SetMaterial` (`self.StaticMeshComponent`) 0 "/Game/Level_Quentin_Dictateur_Supreme/Materials/Flash.Flash")
        (bind _returnvalue (`|CreateWidget` "/Game/Level_Quentin_Dictateur_Supreme/Interface/W_Interface_End.W_Interface_End_C"))
        (`UserWidget.AddToViewport` _returnvalue 0)
        (`GameplayStatics.PlaySound2D` "/Game/Level_Quentin_Dictateur_Supreme/Assets/FlashBange_SoundCue.FlashBange_SoundCue" 1.0 1.0 0.0 null null)
        (`KismetSystemLibrary.Delay` 8.0)
        (`GameplayStatics.OpenLevel` "Level_EndLobby")))))

(fn `UserConstructionScript`)