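; Level dialogue controller that shows dialogue through the player's HUD at game start and in response to two referenced buttons.
; BeginPlay sends the spawn dialogue to CreateDialogue on the HUD.
; Tick polls a flag on each button, giving Bouton2 priority over Bouton14, then shows that button's dialogue and clears the flag.
; Bouton2's handler also sets GivePermissionsDoor to true after creating its dialogue.
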(event `self.ReceiveTick`
  (params (DeltaSeconds :type "Float (single-precision)"))
  (if (`/Game/Level_Quentin_Dictateur_Supreme/BluePrints/BP_Bouton2.IsDown?` (`self.bouton 2`))
    (`self.OnActionButton2`)
    (set `/Game/Level_Quentin_Dictateur_Supreme/BluePrints/BP_Bouton2.IsDown?` false (`self.bouton 2`))
    (elif (`/Game/Level_Quentin_Dictateur_Supreme/BluePrints/BP_Bouton14.Dialogue` (`self.bouton 14`))
      (`self.OnActionButton14`)
      (set `/Game/Level_Quentin_Dictateur_Supreme/BluePrints/BP_Bouton14.Dialogue` false (`self.bouton 14`)))))

(event `self.ReceiveBeginPlay`
  (bind _ashud_ (cast `/Game/Level_Adrien/HUD_` (`PlayerController.GetHUD` (`GameplayStatics.GetPlayerController` 0))))
  (`/Game/Level_Adrien/HUD_.CreateDialogue` _ashud_ (`self.DialogueSpawn`)))

(event `OnActionButton14`
  (bind _ashud_ (cast `/Game/Level_Adrien/HUD_` (`PlayerController.GetHUD` (`GameplayStatics.GetPlayerController` 0))))
  (`/Game/Level_Adrien/HUD_.CreateDialogue` _ashud_ (`self.DialogueOn14`)))

(event `OnActionButton2`
  (bind _ashud_ (cast `/Game/Level_Adrien/HUD_` (`PlayerController.GetHUD` (`GameplayStatics.GetPlayerController` 0))))
  (`/Game/Level_Adrien/HUD_.CreateDialogue` _ashud_ (`self.DialogueOn2`))
  (set `self.GivePermissionsDoor` true))

(fn `UserConstructionScript`)