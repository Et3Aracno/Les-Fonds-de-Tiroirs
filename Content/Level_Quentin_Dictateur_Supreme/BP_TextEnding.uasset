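; BP_TextEnding is an interactive trigger that opens a YouTube video link (a Rickroll) when E is pressed while its box is overlapped.
; Begin and end overlap events on the box toggle an IsOverlapping flag, with no check on which actor overlaps.
; Tick polls the first player controller for the E key, and a DoOnce with no reset keeps the URL from launching again.
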(event `self.Box.OnComponentBeginOverlap`
  (params (OverlappedComponent :type "PrimitiveComponent Object Reference") (OtherActor :type "Actor Object Reference") (OtherComp :type "PrimitiveComponent Object Reference") (OtherBodyIndex :type Integer) (bFromSweep :type Boolean) (SweepResult :type "HitResult Structure (by ref)"))
  (set `self.IsOverlapping?` true))

(event `self.ReceiveTick`
  (params (DeltaSeconds :type "Float (single-precision)"))
  (if (and (`self.IsOverlapping?`) (`PlayerController.IsInputKeyDown` (`GameplayStatics.GetPlayerController` 0) "E"))
    (`/Engine/EditorBlueprintResources/StandardMacros.DoOnce` false
      (:`Completed`
        (`KismetSystemLibrary.LaunchURL` "https://www.youtube.com/watch?v=dQw4w9WgXcQ&list=RDdQw4w9WgXcQ&start_radio=1")))))

(event `self.Box.OnComponentEndOverlap`
  (params (OverlappedComponent :type "PrimitiveComponent Object Reference") (OtherActor :type "Actor Object Reference") (OtherComp :type "PrimitiveComponent Object Reference") (OtherBodyIndex :type Integer))
  (set `self.IsOverlapping?` false))

(fn `UserConstructionScript`)